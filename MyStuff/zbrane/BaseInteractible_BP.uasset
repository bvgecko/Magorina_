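; Base interactible item for pickups and hand-held weapons, loading its ItemInfo from a data table by ItemName.
; Interact, pickup and destroy events call into player character 0.
; Blade and handle (Rukojet) boxes, toggled by WeaponActive/WeaponDeactive and unbound for one item type, deal server-routed damage once per timed swing, the handle at a tenth.
; Heater shield overlaps zero the player's damage, and hits on players count only on HitboxTorso.
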(event `self.ReceiveBeginPlay`
  (bind (_itemclass _itemname _itemimage _currentstack _maxstack _itemindex _itemtype) (break `/Game/MyStuff/zbrane/ItemInfo_S` (`self.ItemInfo`)))
  (if (not (or (`|EnumInequality` _itemtype "NewEnumerator3") (`|EnumEquality` _itemtype "NewEnumerator4")))
    (clear `PrimitiveComponent.OnComponentBeginOverlap` (`self.DmgBox`))
    (clear `PrimitiveComponent.OnComponentBeginOverlap` (`self.RukojetDmgBox`))))

(event `/Game/MyStuff/zbrane/Interact_BPI.DestroyWeaponFromHand`
  (bind _asplayer_base_bp (cast `/Game/MyStuff/PlayerBase_BP` (`GameplayStatics.GetPlayerCharacter` 0)))
  (`/Game/MyStuff/PlayerBase_BP.Destroy weapon server` _asplayer_base_bp self))

(event `/Game/MyStuff/zbrane/Interact_BPI.Interact`
  (bind _asplayer_base_bp (cast `/Game/MyStuff/PlayerBase_BP` (`GameplayStatics.GetPlayerCharacter` 0)))
  (`self.InteractionEvent_MP`)
  (`/Game/MyStuff/PlayerBase_BP.Interact_Destroy_MP_event_server` _asplayer_base_bp self))

(event `/Game/MyStuff/zbrane/Interact_BPI.DestroyShieldFromHand`
  (bind _asplayer_base_bp (cast `/Game/MyStuff/PlayerBase_BP` (`GameplayStatics.GetPlayerCharacter` 0)))
  (`/Game/MyStuff/PlayerBase_BP.Destroy shield server` _asplayer_base_bp self))

(event `InteractionEvent_MP`
  (`/Game/MyStuff/PlayerBase_BP.PickupItem` (stale `/Game/MyStuff/zbrane/Interact_BPI.Interact` _asplayer_base_bp) (`self.ItemInfo`)))

(event `self.DmgBox.OnComponentBeginOverlap`
  (params (OverlappedComponent :type "PrimitiveComponent Object Reference") (OtherActor :type "Actor Object Reference") (OtherComp :type "PrimitiveComponent Object Reference") (OtherBodyIndex :type Integer) (bFromSweep :type Boolean) (SweepResult :type "HitResult Structure (by ref)"))
  (`|ExecutionSequence`
    (:`then_0`
      ;[1 1 1] asi k hovnu
      (bind _asheater_shield_bp (cast `/Game/MyStuff/zbrane/Heater_shield_BP` OtherActor))
      (`KismetSystemLibrary.PrintString` "Zasazen Stit cepeli" true true (struct :`R` 0.085945 :`G` 0.15625 :`B` 0.072812 :`A` 1.0))
      (bind _asplayer_base_bp (cast `/Game/MyStuff/PlayerBase_BP` (`GameplayStatics.GetPlayerCharacter` 0)))
      (set `/Game/MyStuff/PlayerBase_BP.Basic damage` 0.0 _asplayer_base_bp)
      (set `/Game/MyStuff/PlayerBase_BP.DmgUdelen` true _asplayer_base_bp))
    (:`then_1`
      (bind _output_get (set `self.Trefeny actor` OtherActor))
      (cast `/Game/MyStuff/PlayerBase_BP` _output_get
        (:`CastFailed`
          (bind _asplayer_base_bp_2 (cast `/Game/MyStuff/PlayerBase_BP` (`GameplayStatics.GetPlayerCharacter` 0)))
          (bind _output_get_2 (set `self.As Player Base BP` _asplayer_base_bp_2))
          (if (`/Game/MyStuff/PlayerBase_BP.sek?` _output_get_2)
            (if (`/Game/MyStuff/PlayerBase_BP.TimeToDmg` _output_get_2)
              (if (not (`/Game/MyStuff/PlayerBase_BP.DmgUdelen` _output_get_2))
                (set `/Game/MyStuff/PlayerBase_BP.DmgUdelen` true _output_get_2)
                (bind _output_get_3 (set `self.Final damage` (* (`/Game/MyStuff/PlayerBase_BP.Basic damage` _output_get_2) (`self.Weapon Damage koef`))))
                (`KismetSystemLibrary.PrintString` (`KismetStringLibrary.Conv_DoubleToString` _output_get_3) true true (struct :`R` 1.0 :`G` 0.608814 :`A` 1.0))
                (`/Game/MyStuff/PlayerBase_BP.ApplyDamageOnServer` _output_get_2 _output_get _output_get_3 _output_get_2)
                (bind _output_get_4 (set `self.Overlapped Component` OverlappedComponent))
                (`KismetSystemLibrary.PrintString` (`KismetSystemLibrary.GetDisplayName` _output_get_4) true true (struct :`R` 0.924884 :`G` 1.0 :`B` 0.929504 :`A` 1.0))
                (`KismetSystemLibrary.PrintString` (`KismetStringLibrary.Conv_BoolToString` (== _output_get_4 (`self.DmgBox`))) true true (struct :`R` 0.979167 :`G` 1.0 :`B` 1.0 :`A` 1.0))))))))
    (:`then_2`
      (bind _asplayer_base_bp_3 (cast `/Game/MyStuff/PlayerBase_BP` OtherActor))
      (set `self.Ten koho trefim` _asplayer_base_bp_3)
      (bind _asplayer_base_bp_4 (cast `/Game/MyStuff/PlayerBase_BP` (`GameplayStatics.GetPlayerCharacter` 0)))
      (if (== (`.HitComponent` (`GameplayStatics.BreakHitResult` SweepResult)) (`/Game/MyStuff/PlayerBase_BP.HitboxTorso` _asplayer_base_bp_3))
        (if (`/Game/MyStuff/PlayerBase_BP.sek?` _asplayer_base_bp_4)
          (if (`/Game/MyStuff/PlayerBase_BP.TimeToDmg` _asplayer_base_bp_4)
            (if (not (`/Game/MyStuff/PlayerBase_BP.DmgUdelen` _asplayer_base_bp_4))
              (set `/Game/MyStuff/PlayerBase_BP.DmgUdelen` true _asplayer_base_bp_4)
              (bind _output_get_5 (set `self.Final damage` (* (`/Game/MyStuff/PlayerBase_BP.Basic damage` _asplayer_base_bp_4) (`self.Weapon Damage koef`))))
              (`KismetSystemLibrary.PrintString` (`KismetStringLibrary.Conv_DoubleToString` _output_get_5) true true (struct :`R` 0.130208 :`B` 0.068673 :`A` 1.0))
              (`/Game/MyStuff/PlayerBase_BP.ApplyDamageOnServer` _asplayer_base_bp_4 OtherActor _output_get_5 _asplayer_base_bp_4))))))))

(event `self.RukojetDmgBox.OnComponentBeginOverlap`
  (params (OverlappedComponent :type "PrimitiveComponent Object Reference") (OtherActor :type "Actor Object Reference") (OtherComp :type "PrimitiveComponent Object Reference") (OtherBodyIndex :type Integer) (bFromSweep :type Boolean) (SweepResult :type "HitResult Structure (by ref)"))
  (`|ExecutionSequence`
    (:`then_0`
      (bind _asheater_shield_bp (cast `/Game/MyStuff/zbrane/Heater_shield_BP` OtherActor))
      (`KismetSystemLibrary.PrintString` "Zasazen Stit rukojeti" true true (struct :`R` 0.085945 :`G` 0.15625 :`B` 0.072812 :`A` 1.0))
      (bind _asplayer_base_bp (cast `/Game/MyStuff/PlayerBase_BP` (`GameplayStatics.GetPlayerCharacter` 0)))
      (set `/Game/MyStuff/PlayerBase_BP.Basic damage` 0.0 _asplayer_base_bp)
      (set `/Game/MyStuff/PlayerBase_BP.DmgUdelen` true _asplayer_base_bp))
    (:`then_1`
      (bind _output_get (set `self.Trefeny actor` OtherActor))
      (cast `/Game/MyStuff/PlayerBase_BP` _output_get
        (:`CastFailed`
          (bind _asplayer_base_bp_2 (cast `/Game/MyStuff/PlayerBase_BP` (`GameplayStatics.GetPlayerCharacter` 0)))
          (bind _output_get_2 (set `self.As Player Base BP` _asplayer_base_bp_2))
          (if (`/Game/MyStuff/PlayerBase_BP.sek?` _output_get_2)
            (if (`/Game/MyStuff/PlayerBase_BP.TimeToDmg` _output_get_2)
              (if (not (`/Game/MyStuff/PlayerBase_BP.DmgUdelen` _output_get_2))
                (set `/Game/MyStuff/PlayerBase_BP.DmgUdelen` true _output_get_2)
                (bind _output_get_3 (set `self.Final damage` (* (* (`/Game/MyStuff/PlayerBase_BP.Basic damage` _output_get_2) (`self.Weapon Damage koef`)) 0.1)))
                (`KismetSystemLibrary.PrintString` (`KismetStringLibrary.Conv_DoubleToString` _output_get_3) true true (struct :`R` 1.0 :`G` 0.608814 :`A` 1.0))
                (`/Game/MyStuff/PlayerBase_BP.ApplyDamageOnServer` _output_get_2 _output_get _output_get_3 _output_get_2)
                (bind _output_get_4 (set `self.Overlapped Component` OverlappedComponent))
                (`KismetSystemLibrary.PrintString` (`KismetSystemLibrary.GetDisplayName` _output_get_4) true true (struct :`R` 0.924884 :`G` 1.0 :`B` 0.929504 :`A` 1.0))
                (`KismetSystemLibrary.PrintString` (`KismetStringLibrary.Conv_BoolToString` (== _output_get_4 (`self.DmgBox`))) true true (struct :`R` 0.979167 :`G` 1.0 :`B` 1.0 :`A` 1.0))))))))
    (:`then_2`
      (bind _asplayer_base_bp_3 (cast `/Game/MyStuff/PlayerBase_BP` OtherActor))
      (set `self.Ten koho trefim` _asplayer_base_bp_3)
      (bind _asplayer_base_bp_4 (cast `/Game/MyStuff/PlayerBase_BP` (`GameplayStatics.GetPlayerCharacter` 0)))
      (if (== (`.HitComponent` (`GameplayStatics.BreakHitResult` SweepResult)) (`/Game/MyStuff/PlayerBase_BP.HitboxTorso` _asplayer_base_bp_3))
        (if (`/Game/MyStuff/PlayerBase_BP.sek?` _asplayer_base_bp_4)
          (if (`/Game/MyStuff/PlayerBase_BP.TimeToDmg` _asplayer_base_bp_4)
            (if (not (`/Game/MyStuff/PlayerBase_BP.DmgUdelen` _asplayer_base_bp_4))
              (set `/Game/MyStuff/PlayerBase_BP.DmgUdelen` true _asplayer_base_bp_4)
              (bind _output_get_5 (set `self.Final damage` (* (* (`/Game/MyStuff/PlayerBase_BP.Basic damage` _asplayer_base_bp_4) (`self.Weapon Damage koef`)) 0.1)))
              (`KismetSystemLibrary.PrintString` (`KismetStringLibrary.Conv_DoubleToString` _output_get_5) true true (struct :`R` 0.130208 :`G` 0.032402 :`B` 0.011562 :`A` 1.0))
              (`/Game/MyStuff/PlayerBase_BP.ApplyDamageOnServer` _asplayer_base_bp_4 OtherActor _output_get_5 _asplayer_base_bp_4))))))))

(event `WeaponActive`
  (`PrimitiveComponent.SetCollisionProfileName` (`self.DmgBox`) "OverlapAll" true)
  (`PrimitiveComponent.SetCollisionProfileName` (`self.RukojetDmgBox`) "OverlapAll" true))

(event `WeaponDeactive`
  (`PrimitiveComponent.SetCollisionEnabled` (`self.DmgBox`) "NoCollision")
  (`PrimitiveComponent.SetCollisionEnabled` (`self.RukojetDmgBox`) "NoCollision"))

(fn `PickupItems_MP`)

(fn `UserConstructionScript`
  (bind _returnvalue (`|GetDataTableRow` "/Game/MyStuff/zbrane/ItemInfo_DT.ItemInfo_DT" (`KismetStringLibrary.Conv_StringToName` (`|GetEnumeratorNameAsString` (`self.ItemName`))))
    (:`then`
      (set `self.ItemInfo` _returnvalue))))